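; BP_FireSpurt is a fire trap that shows a flame particle effect when the player steps into its trigger box and damages them while they stay in it.
; Begin and end overlap events turn the particle visibility on and off after short delays, reacting only to the player reference cached at BeginPlay.
; Tick checks that the flame is visible and the player still overlaps, then applies damage through a DoOnce that resets after a delay, producing periodic hits.
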(event OnComponentBeginOverlap(TriggerBox)
  (params (OverlappedComponent :type Primitive%20Component%20Object%20Reference) (OtherActor :type Actor%20Object%20Reference) (OtherComp :type Primitive%20Component%20Object%20Reference) (OtherBodyIndex :type Integer) (bFromSweep :type Boolean) (SweepResult :type Hit%20Result%20Structure%20%28by%20ref%29))
  ;[0 0 0 0.5] Activate Fire
  (if (== OtherActor (Variables|Default|GetPlayer%20Ref))
    (Utilities|FlowControl|Delay 0.25)
    (Rendering|SetVisibility (Variables|Default|GetParticleSystem) true false)))

(event OnComponentEndOverlap(TriggerBox)
  (params (OverlappedComponent :type Primitive%20Component%20Object%20Reference) (OtherActor :type Actor%20Object%20Reference) (OtherComp :type Primitive%20Component%20Object%20Reference) (OtherBodyIndex :type Integer))
  ;[0 0 0 0.5] Deactivate Fire
  (if (== OtherActor (Variables|Default|GetPlayer%20Ref))
    (Utilities|FlowControl|Delay 1.0)
    (Rendering|SetVisibility (Variables|Default|GetParticleSystem) false false)))

(event EventBeginPlay
  ;[0 0 0 0.5] Create Player Ref
  (bind _asbp_third_person_character (Utilities|Casting|CastToBP_ThirdPersonCharacter (Game|GetPlayerCharacter 0)))
  (Variables|Default|SetPlayer%20Ref _asbp_third_person_character))

(event EventTick
  (params (DeltaSeconds :type Float%20%28single-precision%29))
  ;[0 0 0 0.5] Apply Damage To Player
  (if (and (Rendering|IsVisible (Variables|Default|GetParticleSystem)) (Collision|IsOverlappingActor (Variables|Default|GetTrigger%20Box) (Variables|Default|GetPlayer%20Ref) :!class /Script/Engine.PrimitiveComponent))
    (Utilities|FlowControl|DoOnce false :!label _label
      (:Completed
        (Game|Damage|ApplyDamage (Variables|Default|GetPlayer%20Ref) (Variables|Default|GetDamageAmount) 0 0)
        (Utilities|FlowControl|Delay 1.0)
        (goto _label Reset)))))

(fn ConstructionScript)