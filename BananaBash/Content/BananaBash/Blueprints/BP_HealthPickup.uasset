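; BP_HealthPickup is a pickup that restores health to the player when touched.
; On BeginPlay it caches the player character cast to BP_ThirdPersonCharacter.
; When that player overlaps TriggerSphere, it adds HealthAddAmount to CurrentHealth clamped to a fixed range, prints the new value, and destroys itself.
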(event OnComponentBeginOverlap(TriggerSphere)
  (params (OverlappedComponent :type Primitive%20Component%20Object%20Reference) (OtherActor :type Actor%20Object%20Reference) (OtherComp :type Primitive%20Component%20Object%20Reference) (OtherBodyIndex :type Integer) (bFromSweep :type Boolean) (SweepResult :type Hit%20Result%20Structure%20%28by%20ref%29))
  (bind _player_ref (Variables|Default|GetPlayer%20Ref))
  ;[0 0 0 0.5] Add Health To Player
  (if (== OtherActor _player_ref)
    (bind _output_get (Variables|/Game/BananaBash/Blueprints/BP_ThirdPersonCharacter.BP_ThirdPersonCharacter_C|SetCurrentHealth _player_ref (Math|Float|Clamp(Float) (+ (Variables|/Game/BananaBash/Blueprints/BP_ThirdPersonCharacter.BP_ThirdPersonCharacter_C|GetCurrentHealth _player_ref) (Variables|Default|GetHealthAddAmount)) 0.0 1e+02)))
    (Development|PrintString (Utilities|String|ToString(Float) _output_get))
    (Actor|DestroyActor)))

(event EventBeginPlay
  ;[0 0 0 0.5] Create Player Ref
  (bind _asbp_third_person_character (Utilities|Casting|CastToBP_ThirdPersonCharacter (Game|GetPlayerCharacter 0)))
  (Variables|Default|SetPlayer%20Ref _asbp_third_person_character))

(fn ConstructionScript)