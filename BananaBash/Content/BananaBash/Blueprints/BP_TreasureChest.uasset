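; BP_TreasureChest is a chest that opens once when the player walks into its box trigger and throws out a health pickup.
; The player character is cached on BeginPlay to filter the overlap, and a DoOnce starts the OpenLid timeline that rotates the lid on its roll axis.
; When the timeline finishes, a BP_HealthPickup spawns at SpawnPos with physics enabled and gets an impulse forward and mostly upward.
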(event OnComponentBeginOverlap(Box)
  (params (OverlappedComponent :type Primitive%20Component%20Object%20Reference) (OtherActor :type Actor%20Object%20Reference) (OtherComp :type Primitive%20Component%20Object%20Reference) (OtherBodyIndex :type Integer) (bFromSweep :type Boolean) (SweepResult :type Hit%20Result%20Structure%20%28by%20ref%29))
  (bind _lid (Variables|Default|GetLid))
  (bind _relativerotation (Variables|/Script/Engine.SceneComponent|GetRelativeRotation _lid))
  ;[0 0 0 0.5] Open Chest Animation
  (if (== OtherActor (Variables|Default|GetPlayer%20Ref))
    (Utilities|FlowControl|DoOnce false
      (:Completed
        (bind _xrotation (Timeline|Open%20Lid Play)
          (:Update
            (Transformation|SetRelativeRotation _lid (Math|Rotator|MakeRotator _xrotation (.pitch _relativerotation) (.yaw _relativerotation)) false false))
          (:Finished
            ;[0 0 0 0.5] Spawn Items
            (bind _returnvalue (Game|SpawnActorfromClass "/Game/BananaBash/Blueprints/BP_HealthPickup.BP_HealthPickup_C" (Transformation|GetWorldTransform (Variables|Default|GetSpawnPos)) "Undefined" "MultiplyWithRoot" 0 0))
            (Physics|SetSimulatePhysics (Variables|/Game/BananaBash/Blueprints/BP_HealthPickup.BP_HealthPickup_C|GetSphere _returnvalue) true)
            (Physics|AddImpulseatLocation (Variables|/Game/BananaBash/Blueprints/BP_HealthPickup.BP_HealthPickup_C|GetSphere _returnvalue) (+ (* (Transformation|GetActorForwardVector) 1e+03) (* (Transformation|GetActorUpVector) 4e+03)) (Transformation|GetActorLocation _returnvalue) "None")))))))

(event EventBeginPlay
  ;[0 0 0 0.5] Create Player Ref
  (bind _asbp_third_person_character (Utilities|Casting|CastToBP_ThirdPersonCharacter (Game|GetPlayerCharacter 0)))
  (Variables|Default|SetPlayer%20Ref _asbp_third_person_character))

(fn ConstructionScript)