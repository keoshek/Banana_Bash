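; BP_FallingBlock is a block that drops when the player character enters its trigger box, then rises again.
; Overlap starts the BlockFall timeline after a short delay, and BlockRise follows after a longer pause.
; Both timelines set the mesh's absolute world Z, keeping X and Y.
; An Animating flag blocks re-triggering mid-cycle, and the cycle repeats if the player is still inside when the rise finishes.
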(event OnComponentBeginOverlap(TriggerBox)
  (params (OverlappedComponent :type Primitive%20Component%20Object%20Reference) (OtherActor :type Actor%20Object%20Reference) (OtherComp :type Primitive%20Component%20Object%20Reference) (OtherBodyIndex :type Integer) (bFromSweep :type Boolean) (SweepResult :type Hit%20Result%20Structure%20%28by%20ref%29))
  (bind _staticmesh (Variables|Default|GetStaticMesh))
  (bind _staticmesh_2 (Variables|Default|GetStaticMesh))
  (bind _returnvalue (Transformation|GetWorldLocation _staticmesh))
  (bind _returnvalue_2 (Transformation|GetWorldLocation _staticmesh_2))
  ;[0 0 0 0.5] Block Fall
  (if (and (== OtherActor (Variables|Default|GetPlayer%20Ref)) (not (Variables|Default|GetAnimating)))
    (Variables|Default|SetAnimating true :!label _label)
    (Utilities|FlowControl|Delay 0.2)
    (bind _zheight (Timeline|BlockFall PlayFromStart)
      (:Update
        (Transformation|SetWorldLocation _staticmesh_2 (Math|Vector|MakeVector (.x _returnvalue_2) (.y _returnvalue_2) _zheight) false false))
      (:Finished
        ;[0 0 0 0.5] Block Rise
        (Utilities|FlowControl|Delay 1.0)
        (bind _zheight_2 (Timeline|BlockRise PlayFromStart)
          (:Update
            (Transformation|SetWorldLocation _staticmesh (Math|Vector|MakeVector (.x _returnvalue) (.y _returnvalue) _zheight_2) false false))
          (:Finished
            (Variables|Default|SetAnimating false)
            ;[0 0 0 0.5] Block Fall
            (if (Collision|IsOverlappingActor (Variables|Default|GetTrigger%20Box) (Variables|Default|GetPlayer%20Ref) :!class /Script/Engine.PrimitiveComponent)
              (goto _label))))))))

(event EventBeginPlay
  ;[0 0 0 0.5] Create Player Ref
  (bind _asbp_third_person_character (Utilities|Casting|CastToBP_ThirdPersonCharacter (Game|GetPlayerCharacter 0)))
  (Variables|Default|SetPlayer%20Ref _asbp_third_person_character))

(fn ConstructionScript)