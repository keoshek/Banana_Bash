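; BP_Button is a pressure button that opens and closes a linked gate when the player steps on or off it.
; Trigger sphere overlaps with the cached player character set the pressed state and play the Press timeline forward or in reverse to move the cylinder vertically.
; When the timeline finishes, it opens GateRef if pressed, otherwise closes it after a retriggerable delay if still unpressed.
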(event OnComponentBeginOverlap(TriggerSphere)
  (params (OverlappedComponent :type Primitive%20Component%20Object%20Reference) (OtherActor :type Actor%20Object%20Reference) (OtherComp :type Primitive%20Component%20Object%20Reference) (OtherBodyIndex :type Integer) (bFromSweep :type Boolean) (SweepResult :type Hit%20Result%20Structure%20%28by%20ref%29))
  (bind _cylinder (Variables|Default|GetCylinder))
  (bind _gate_ref (Variables|Default|GetGate%20Ref))
  (bind _relativelocation (Variables|/Script/Engine.SceneComponent|GetRelativeLocation _cylinder))
  ;[0 0 0 0.5] Button Animations
  (if (== OtherActor (Variables|Default|GetPlayer%20Ref))
    (Variables|Default|SetisButtonPressed true)
    (bind _zheight (Timeline|Press PlayFromStart)
      (:Update
        (Transformation|SetRelativeLocation _cylinder (Math|Vector|MakeVector (.x _relativelocation) (.y _relativelocation) _zheight) false false))
      (:Finished
        ;[0 0 0 0.5] Open/Close the Gate
        (Utilities|IsValid _gate_ref
          (:Is%20Valid
            (if (Variables|Default|GetisButtonPressed)
              (Default|OpenGate _gate_ref)
              (else
                (Utilities|FlowControl|RetriggerableDelay (Variables|Default|GetWaitDuration))
                (if (not (Variables|Default|GetisButtonPressed))
                  (Default|CloseGate _gate_ref))))))))))

(event OnComponentEndOverlap(TriggerSphere)
  (params (OverlappedComponent :type Primitive%20Component%20Object%20Reference) (OtherActor :type Actor%20Object%20Reference) (OtherComp :type Primitive%20Component%20Object%20Reference) (OtherBodyIndex :type Integer))
  (bind _cylinder (Variables|Default|GetCylinder))
  (bind _gate_ref (Variables|Default|GetGate%20Ref))
  (bind _relativelocation (Variables|/Script/Engine.SceneComponent|GetRelativeLocation _cylinder))
  ;[0 0 0 0.5] Button Animations
  (if (== OtherActor (Variables|Default|GetPlayer%20Ref))
    (Variables|Default|SetisButtonPressed false)
    (bind _zheight (Timeline|Press ReverseFromEnd)
      (:Update
        (Transformation|SetRelativeLocation _cylinder (Math|Vector|MakeVector (.x _relativelocation) (.y _relativelocation) _zheight) false false))
      (:Finished
        ;[0 0 0 0.5] Open/Close the Gate
        (Utilities|IsValid _gate_ref
          (:Is%20Valid
            (if (Variables|Default|GetisButtonPressed)
              (Default|OpenGate _gate_ref)
              (else
                (Utilities|FlowControl|RetriggerableDelay (Variables|Default|GetWaitDuration))
                (if (not (Variables|Default|GetisButtonPressed))
                  (Default|CloseGate _gate_ref))))))))))

(event EventBeginPlay
  ;[0 0 0 0.5] Create Player Ref
  (bind _asbp_third_person_character (Utilities|Casting|CastToBP_ThirdPersonCharacter (Game|GetPlayerCharacter 0)))
  (Variables|Default|SetPlayer%20Ref _asbp_third_person_character))

(fn ConstructionScript)